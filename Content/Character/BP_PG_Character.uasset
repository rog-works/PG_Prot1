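; Player character that manages the HUD, interact prompt, inventory, active save point, shooting and jump-stat reporting.
; BeginPlay creates widgets, Inventory and NoticeQueue, then binds save-point selection and item-pickup events.
; Tick projects the interact prompt onto the target actor and spawns stacked pickup notices from the queue, releasing slots on destroy.
; Firing aims bullets from ShootArrow toward a camera line-trace point; jumping reports a stat record to BP_GameMode.
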(event OnComponentBeginOverlap(CapsuleComponent)
  (params (OverlappedComponent :type Primitive%20Component%20Object%20Reference) (OtherActor :type Actor%20Object%20Reference) (OtherComp :type Primitive%20Component%20Object%20Reference) (OtherBodyIndex :type Integer) (bFromSweep :type Boolean) (SweepResult :type Hit%20Result%20Structure%20%28by%20ref%29))
  ;[1 1 1] TickよりOverlapの方がコストは小さいが、オブジェクトの座標上に出す場合はTickにしなければならない
)

(event OnComponentEndOverlap(CapsuleComponent)
  (params (OverlappedComponent :type Primitive%20Component%20Object%20Reference) (OtherActor :type Actor%20Object%20Reference) (OtherComp :type Primitive%20Component%20Object%20Reference) (OtherBodyIndex :type Integer))
  ;[1 1 1] TickよりOverlapの方がコストは小さいが、オブジェクトの座標上に出す場合はTickにしなければならない
)

(event Custom|カスタムイベント
  (params (savepoint :type BP%20Save%20Point%20Object%20Reference))
  (CallFunction|SetActiveSavePoint savepoint))

(event Custom|カスタムイベント_0
  (params (item :type Item%20Object%20Reference) (number :type Integer))
  (Default|AddItem (Variables|Default|GetInventory) item number)
  (Default|AddNotice (Variables|Default|GetNoticeQueue) item))

(event Custom|カスタムイベント_1
  (params (signature :type String))
  (Default|EndNotice (Variables|Default|GetNoticeQueue) signature))

(event Input|EnhancedActionEvents|EnhancedInputActionIA_Fire
  (params (ActionValue :type Boolean) (ElapsedSeconds :type Float%20%28double-precision%29) (TriggeredSeconds :type Float%20%28double-precision%29) (InputAction :type Input%20Action%20Object%20Reference :default "/Game/Input/IA_Fire.IA_Fire"))
  (bind _returnvalue (Game|GetPlayerCameraManager 0))
  (bind _shootarrow (Variables|Default|GetShootArrow))
  (bind _returnvalue_2 (Camera|GetCameraLocation _returnvalue))
  (bind _returnvalue_3 (Camera|GetCameraRotation _returnvalue))
  (bind _returnvalue_4 (Transformation|GetSocketLocation _shootarrow "None"))
  (bind _returnvalue_5 (Math|Vector|GetForwardVector _returnvalue_3))
  (bind _returnvalue_6 (* _returnvalue_5 "5000.000000,5000.000000,5000.000000"))
  (bind _returnvalue_7 (+ _returnvalue_6 _returnvalue_2))
  (:Started
    (bind _returnvalue_8 (Game|SpawnActorfromClass "/Game/Object/BP_Bullet.BP_Bullet_C" (Math|Transform|MakeTransform _returnvalue_4 _returnvalue_3 "1.000000,1.000000,1.000000") "Undefined" 0 0))
    (bind (_outhit _returnvalue_9) (Collision|LineTraceByChannel _returnvalue_2 _returnvalue_7 "TraceTypeQuery1" false 0 "None"))
    (if _returnvalue_9
      (Variables|Default|SetTargetLocation (.location _outhit))
      (else
        (Variables|Default|SetTargetLocation _returnvalue_7)))
    (Variables|/Script/Engine.MovementComponent|SetVelocity (Actor|GetComponentbyClass _returnvalue_8 "/Script/Engine.ProjectileMovementComponent") (* (Math|Vector|Normalize (- (Variables|Default|GetTargetLocation) _returnvalue_4)) (Math|Vector|MakeVector (Variables|/Script/Engine.ProjectileMovementComponent|GetInitialSpeed (Actor|GetComponentbyClass _returnvalue_8 "/Script/Engine.ProjectileMovementComponent")) (Variables|/Script/Engine.ProjectileMovementComponent|GetInitialSpeed (Actor|GetComponentbyClass _returnvalue_8 "/Script/Engine.ProjectileMovementComponent")) (Variables|/Script/Engine.ProjectileMovementComponent|GetInitialSpeed (Actor|GetComponentbyClass _returnvalue_8 "/Script/Engine.ProjectileMovementComponent")))))))

(event Input|EnhancedActionEvents|EnhancedInputActionIA_Jump
  (params (ActionValue :type Boolean) (ElapsedSeconds :type Float%20%28double-precision%29) (TriggeredSeconds :type Float%20%28double-precision%29) (InputAction :type Input%20Action%20Object%20Reference :default "/Game/Input/IA_Jump.IA_Jump"))
  (:Started
    (bind _asbp_game_mode (Utilities|Casting|CastToBP_GameMode (Game|GetGameMode)))
    (bind _returnvalue (Game|ConstructObjectfromClass "/Game/Framework/Statistics/StatRecords/StatRecord_PlayerJumps.StatRecord_PlayerJumps_C"))
    (bind _path (Default|CallPath _returnvalue self))
    (Default|OnActivityイベント _asbp_game_mode _path)))

(event EventBeginPlay
  (Utilities|FlowControl|Sequence
    (:then_0
      (bind _returnvalue (UserInterface|CreateWidget "/Game/UI/Game/UI_Interact.UI_Interact_C"))
      (UserInterface|Viewport|AddtoViewport _returnvalue 0)
      (Widget|SetVisibility _returnvalue "Visible")
      (Variables|Default|SetUIInteract _returnvalue))
    (:then_1
      (Utilities|IsValid (Variables|Default|GetActivateSavePoint)
        (:Is%20Not%20Valid
          (bind _outactors (Actor|GetAllActorsOfClass "/Game/Object/BP_SavePoint.BP_SavePoint_C"))
          (for _array_element _outactors
            (if (== (Utilities|GetDisplayName _array_element) "BP_SavePoint")
              (CallFunction|SetActiveSavePoint _array_element))))))
    (:then_2
      (EventDispatchers|BindEventtoOnSelectedSavePoint (delegate Custom|カスタムイベント)))
    (:then_3
      (bind _returnvalue_2 (Game|ConstructObjectfromClass "/Game/Framework/Inventory/Inventory.Inventory_C"))
      (Default|Initialize _returnvalue_2)
      (Variables|Default|SetInventory _returnvalue_2))
    (:then_4
      (bind _returnvalue_3 (UserInterface|CreateWidget "/Game/UI/Game/UI_HUD.UI_HUD_C"))
      (UserInterface|Viewport|AddtoViewport _returnvalue_3 0)
      (Variables|Default|SetUIHud _returnvalue_3))
    (:then_5
      (EventDispatchers|BindEventtoOnGatItem (delegate Custom|カスタムイベント_0)))
    (:then_6
      (bind _returnvalue_4 (Game|ConstructObjectfromClass "/Game/UI/Item/NoticeQueue.NoticeQueue_C"))
      (Variables|Default|SetNoticeQueue _returnvalue_4))))

(event EventTick
  (params (DeltaSeconds :type Float%20%28single-precision%29))
  (bind _uiinteract (Variables|Default|GetUIInteract))
  (bind _actorinteractable (Variables|Default|GetActorInteractable))
  (Utilities|FlowControl|Sequence
    (:then_0
      (Utilities|IsValid _actorinteractable
        (:Is%20Valid
          (Widget|SetVisibility _uiinteract "Visible")
          (Class|Widget|SetRenderTranslation _uiinteract (.ScreenPosition (Class|WidgetLayoutLibrary|ProjectWorldLocationtoWidgetPosition (Game|GetPlayerController 0) (Transformation|GetActorLocation _actorinteractable) false))))
        (:Is%20Not%20Valid
          (Widget|SetVisibility (Variables|Default|GetUIInteract) "Hidden"))))
    (:then_1
      (bind (_activatekey _item) (Default|ProcessQueue (Variables|Default|GetNoticeQueue)))
      (if (> (Utilities|String|Len _activatekey) 0)
        (bind _returnvalue (UserInterface|CreateWidget "/Game/UI/Item/UI_NoticeEntry.UI_NoticeEntry_C"))
        (bind _name (Default|Name _item))
        (Variables|/Game/UI/Item/UI_NoticeEntry.UI_NoticeEntry_C|Settitle _returnvalue _name)
        (Variables|/Game/UI/Item/UI_NoticeEntry.UI_NoticeEntry_C|Setsignature _returnvalue _activatekey)
        (Class|Widget|SetRenderTranslation _returnvalue (Math|Vector2D|MakeVector2D 5e+01 (Math|Conversions|ToFloat(Integer) (+ (* (Math|Conversions|ToInteger(Byte) _activatekey) 64) 200))))
        (UserInterface|Viewport|AddtoViewport _returnvalue 0)
        (EventDispatchers|BindEventtoOnDestroy _returnvalue (delegate Custom|カスタムイベント_1))))))

(fn ConstructionScript)

(fn SetActiveSavePoint
  (params (savepoint :type BP%20Save%20Point%20Object%20Reference))
  (if (!= savepoint (Variables|Default|GetActivateSavePoint))
    (Utilities|FlowControl|Sequence
      (:then_0
        (Utilities|IsValid (Variables|Default|GetActivateSavePoint)
          (:Is%20Valid
            (Default|CallOnActivated (Variables|Default|GetActivateSavePoint) false))))
      (:then_1
        (bind _output_get (Variables|Default|SetActivateSavePoint savepoint))
        (Default|CallOnActivated _output_get true)))))