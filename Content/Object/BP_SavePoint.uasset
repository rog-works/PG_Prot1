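; BP_SavePoint is an interactable save point that reports itself to the player character as selected.
; The construction script tints a dynamic emissive material on its cylinder and shows the initial activated state.
; An activation event toggles the glow through TurnLightOn and plays a sound when switched on.
; On activation it also builds a per-save-point stat record and sends it to the game mode as activity.
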(event Custom|OnInteract_イベント
  (params (On :type Boolean))
  (if On
    (bind _asbp_pg_character (Utilities|Casting|CastToBP_PG_Character (Game|GetPlayerCharacter 0)))
    (Default|CallOnSelectedSavePoint _asbp_pg_character self)))

(event Custom|カスタムイベント_0
  (params (On :type Boolean))
  (Utilities|FlowControl|Sequence
    (:then_0
      (bind _output_get (Variables|Default|SetActivated On))
      (CallFunction|TurnLighton _output_get)
      (if _output_get
        (Audio|PlaySound2D "/Game/Resources/External/SoundEffectLab/SE_SavePoint_Cue.SE_SavePoint_Cue" 1.0 1.0 0.0 0 0)))
    (:then_1
      (if On
        (bind _asbp_game_mode (Utilities|Casting|CastToBP_GameMode (Game|GetGameMode)))
        (bind _returnvalue (Game|ConstructObjectfromClass "/Game/Framework/Statistics/StatRecords/StatRecord_PerSavePointActivates.StatRecord_PerSavePointActivates_C"))
        (bind _path (Default|CallPath _returnvalue self))
        (Default|CallOnActivity _asbp_game_mode _path)))))

(event EventBeginPlay
  (Utilities|FlowControl|Sequence
    (:then_0
      (EventDispatchers|AssignOnInteract (delegate Custom|OnInteract_イベント)))
    (:then_1
      (EventDispatchers|BindEventtoOnActivated (delegate Custom|カスタムイベント_0)))))

(fn ConstructionScript
  (bind _returnvalue (Rendering|Material|CreateDynamicMaterialInstance (Variables|Default|GetCylinder) 0 0 "None" :!class /Script/Engine.PrimitiveComponent))
  (Rendering|Material|SetVectorParameterValue _returnvalue "EmissiveColor" (LocalVariables|Getcolor) :!class /Script/Engine.MaterialInstanceDynamic)
  (Variables|Default|SetMI_Light _returnvalue)
  (CallFunction|TurnLighton (Variables|Default|GetActivated)))

(fn TurnLighton
  (params (On :type Boolean))
  (bind _mi_light (Variables|Default|GetMI_Light))
  (if On
    (Rendering|Material|SetScalarParameterValue _mi_light "EmissivePower" 1e+01 :!class /Script/Engine.MaterialInstanceDynamic)
    (else
      (Rendering|Material|SetScalarParameterValue _mi_light "EmissivePower" 0.0 :!class /Script/Engine.MaterialInstanceDynamic))))