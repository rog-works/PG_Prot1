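; BP_Switch is a toggle switch that drives a linked Mover, with a lit button showing its on/off state.
; Interacting through PGInteract, bound only when a Mover is valid, flips the state and runs ProcessMove, which extends the parent, updates the light with a click sound and moves the Mover.
; A BP_Bullet entering the sphere passes the inverted state to TurnComponent.
; The light uses a dynamic material's EmissivePower, initialized silently in construction.
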(event OnComponentBeginOverlap(Sphere)
  (params (OverlappedComponent :type Primitive%20Component%20Object%20Reference) (OtherActor :type Actor%20Object%20Reference) (OtherComp :type Primitive%20Component%20Object%20Reference) (OtherBodyIndex :type Integer) (bFromSweep :type Boolean) (SweepResult :type Hit%20Result%20Structure%20%28by%20ref%29))
  (Utilities|Casting|CastToBP_Bullet OtherActor)
  (Default|Turnon (Variables|Default|GetTurnComponent) (not (Variables|Default|Geton))))

(event Custom|OnInteract_イベント_0
  (params (On :type Boolean))
  (bind _output_get (Variables|Default|Seton (not (Variables|Default|Geton))))
  (CallFunction|ProcessMove _output_get))

(event EventBeginPlay
  (|CallParentFunction)
  (Utilities|IsValid (Variables|Default|Getmover)
    (:Is%20Valid
      (EventDispatchers|AssignOnInteract (Variables|Default|GetPG_Interact) (delegate Custom|OnInteract_イベント_0)))))

(fn ConstructionScript
  (bind _returnvalue (Rendering|Material|CreateDynamicMaterialInstance (Variables|Default|Getbutton) 0 0 "None" :!class /Script/Engine.PrimitiveComponent))
  (Variables|Default|SetMI_Light _returnvalue)
  (CallFunction|TurnLighton (Variables|Default|Geton) false))

(fn TurnLighton
  (params (on :type Boolean) (playSE :type Boolean))
  (bind _mi_light (Variables|Default|GetMI_Light))
  (if playSE
    (Audio|PlaySound2D "/Game/Resources/External/SoundEffectLab/SE_Click_Cue.SE_Click_Cue" 1.0 1.0 0.0 0 0))
  (if on
    (Rendering|Material|SetScalarParameterValue _mi_light "EmissivePower" 1.0 :!class /Script/Engine.MaterialInstanceDynamic)
    (else
      (Rendering|Material|SetScalarParameterValue _mi_light "EmissivePower" 0.0 :!class /Script/Engine.MaterialInstanceDynamic))))

(fn ProcessMove
  (params (on :type Boolean))
  (|CallParentFunction on)
  (CallFunction|TurnLighton on true)
  (Default|Move (Variables|Default|Getmover) on))