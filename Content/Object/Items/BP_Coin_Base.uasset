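; BP_Coin_Base is a base coin pickup that gives an item to the BP_PG_Character overlapping its sphere.
; On overlap it constructs an ItemClass object, passes it with Amount to the character, spawns BP_NS_Coin, plays a sound and destroys itself.
; A timeline that restarts itself on finish drives the coin's rotation through a full turn.
; The construction script tints a dynamic metal material on the cylinder with BaseColor.
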(event OnComponentBeginOverlap(Sphere)
  (params (OverlappedComponent :type Primitive%20Component%20Object%20Reference) (OtherActor :type Actor%20Object%20Reference) (OtherComp :type Primitive%20Component%20Object%20Reference) (OtherBodyIndex :type Integer) (bFromSweep :type Boolean) (SweepResult :type Hit%20Result%20Structure%20%28by%20ref%29))
  (bind _asbp_pg_character (Utilities|Casting|CastToBP_PG_Character OtherActor))
  (bind _returnvalue (Game|ConstructObjectfromClass (Variables|Default|GetitemClass)))
  (Default|CallOnGatItem _asbp_pg_character _returnvalue (Variables|Default|GetAmount))
  (Game|SpawnActorfromClass "/Game/Effect/BP_NS_Coin.BP_NS_Coin_C" (Transformation|GetActorTransform) "Undefined" 0 0)
  (Audio|PlaySound2D "/Game/Resources/External/SoundEffectLab/SE_Coin.SE_Coin" 1.0 1.0 0.0 0 0)
  (Actor|DestroyActor))

(event Custom|RollStart
  (bind _新規track_0 (Timeline|タイムライン PlayFromStart)
    (:Update
      (Transformation|SetActorRotation (Math|Rotator|Lerp(Rotator) "0, 0, 0" "0.000000,360.000000,0.000000" _新規track_0)))
    (:Finished
      (CallFunction|RollStart))))

(event EventBeginPlay
  (CallFunction|RollStart))

(fn ConstructionScript
  (bind _returnvalue (Rendering|Material|CreateDynamicMaterialInstance (Variables|Default|GetCylinder) 0 "/Game/Object/M_Metal.M_Metal" "None" :!class /Script/Engine.PrimitiveComponent))
  (Rendering|Material|SetVectorParameterValue _returnvalue "Color" (Variables|Default|GetBaseColor) :!class /Script/Engine.MaterialInstanceDynamic))