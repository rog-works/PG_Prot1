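; Base pickup item that grants a quantity of an item class to a character and stays collected once recorded.
; Pickup calls the character's get-item handler, spawns a coin effect, plays a sound, destroys itself and reports a discovery to BP_GameMode.
; After load completes, it destroys itself if its object path, split at the last dot, is in those discovery records.
; RollStart loops a timeline-driven spin.
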(event Custom|RollStart
  (bind _新規track_0 (Timeline|タイムライン PlayFromStart)
    (:Update
      (Transformation|SetActorRotation (Math|Rotator|Lerp(Rotator) "0, 0, 0" "0.000000,360.000000,0.000000" _新規track_0)))
    (:Finished
      (CallFunction|RollStart))))

(event Custom|OnLoadCompleted_イベント_0
  (bind _casspawn (CallFunction|CanSpawn))
  (if (not _casspawn)
    (Actor|DestroyActor)))

(event EventBeginPlay
  (bind _asbp_game_mode (Utilities|Casting|CastToBP_GameMode (Game|GetGameMode)))
  (EventDispatchers|AssignOnLoadCompleted _asbp_game_mode (delegate Custom|OnLoadCompleted_イベント_0)))

(fn ConstructionScript)

(fn ProcessGetItem
  (params (character :type BP%20PG%20Character%20Object%20Reference))
  (Utilities|FlowControl|Sequence
    (:then_0
      (bind _returnvalue (Game|ConstructObjectfromClass (Variables|Default|GetitemClass)))
      (Default|CallOnGatItem character _returnvalue (Variables|Default|Getquantity))
      (Game|SpawnActorfromClass "/Game/Effect/BP_NS_Coin.BP_NS_Coin_C" (Transformation|GetActorTransform) "Undefined" 0 0)
      (Audio|PlaySound2D "/Game/Resources/External/SoundEffectLab/SE_Coin.SE_Coin" 1.0 1.0 0.0 0 0)
      (Actor|DestroyActor))
    (:then_1
      (bind _asbp_game_mode (Utilities|Casting|CastToBP_GameMode (Game|GetGameMode)))
      (bind _returnvalue_2 (Game|ConstructObjectfromClass "/Game/Framework/Statistics/StatRecords/StatRecord_ObjectSymbolDiscovery.StatRecord_ObjectSymbolDiscovery_C"))
      (bind _path (Default|CallPath _returnvalue_2 self))
      (Default|OnActivityイベント _asbp_game_mode _path))))

(fn CanSpawn
  (bind _asbp_game_mode (Utilities|Casting|CastToBP_GameMode (Game|GetGameMode))
    (:then
      (bind _returnvalue (Game|ConstructObjectfromClass "/Game/Framework/Statistics/StatRecords/StatRecord_ObjectSymbolDiscovery.StatRecord_ObjectSymbolDiscovery_C"))
      (bind _path (Default|CallPath _returnvalue self))
      (if (.ReturnValue (Utilities|Map|Find (Variables|/Game/Framework/Statistics/Statistics.Statistics_C|Getrecords (Variables|/Game/Framework/BP_GameMode.BP_GameMode_C|GetStatistics _asbp_game_mode)) (.LeftS (Utilities|String|Split _path "." "IgnoreCase" "FromEnd"))))
        (bind _asstat_record_object_symbol_discovery (Utilities|Casting|CastToStatRecord_ObjectSymbolDiscovery (.Value (Utilities|Map|Find (Variables|/Game/Framework/Statistics/Statistics.Statistics_C|Getrecords (Variables|/Game/Framework/BP_GameMode.BP_GameMode_C|GetStatistics _asbp_game_mode)) (.LeftS (Utilities|String|Split _path "." "IgnoreCase" "FromEnd"))))))
        (return (< (Utilities|Array|FindItem (Variables|/Game/Framework/Statistics/StatRecords/StatRecord_ObjectSymbolDiscovery.StatRecord_ObjectSymbolDiscovery_C|Getdiscoveries _asstat_record_object_symbol_discovery) (.RightS (Utilities|String|Split _path "." "IgnoreCase" "FromEnd"))) 0))
        (else
          (return true))))
    (:CastFailed
      (return true))))