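; BP_Gravity is a toggleable low-gravity zone for BP_PG_Character.
; Box overlap events set the character's movement GravityScale low on entry and to a fixed higher value on exit, rather than restoring the previous one.
; Move stores the On state and calls SetRange, which also runs at construction.
; SetRange switches the zone by sizing the box to Range or collapsing it to zero, updating overlaps.
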(event OnComponentBeginOverlap(Box)
  (params (OverlappedComponent :type Primitive%20Component%20Object%20Reference) (OtherActor :type Actor%20Object%20Reference) (OtherComp :type Primitive%20Component%20Object%20Reference) (OtherBodyIndex :type Integer) (bFromSweep :type Boolean) (SweepResult :type Hit%20Result%20Structure%20%28by%20ref%29))
  (bind _asbp_pg_character (Utilities|Casting|CastToBP_PG_Character OtherActor))
  (Variables|/Script/Engine.CharacterMovementComponent|SetGravityScale (Actor|GetComponentbyClass _asbp_pg_character "/Script/Engine.CharacterMovementComponent") 0.15))

(event OnComponentEndOverlap(Box)
  (params (OverlappedComponent :type Primitive%20Component%20Object%20Reference) (OtherActor :type Actor%20Object%20Reference) (OtherComp :type Primitive%20Component%20Object%20Reference) (OtherBodyIndex :type Integer))
  (bind _asbp_pg_character (Utilities|Casting|CastToBP_PG_Character OtherActor))
  (Variables|/Script/Engine.CharacterMovementComponent|SetGravityScale (Actor|GetComponentbyClass _asbp_pg_character "/Script/Engine.CharacterMovementComponent") 1.5))

(fn ConstructionScript
  (CallFunction|SetRange (Variables|Default|Geton)))

(fn Move
  (params (on :type Boolean))
  (bind _output_get (Variables|Default|Seton on))
  (CallFunction|SetRange _output_get))

(fn SetRange
  (params (on :type Boolean))
  (bind _box (Variables|Default|GetBox))
  (if on
    (Components|Box|SetBoxExtent _box (Variables|Default|GetRange) true)
    (else
      (Components|Box|SetBoxExtent _box "0, 0, 0" true))))