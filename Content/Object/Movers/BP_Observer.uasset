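; BP_Observer links a set of triggers to a mover, so the mover responds to whether every trigger is on.
; At BeginPlay it binds to the OnTurned event of each entry in Triggers.
; Each event recounts the triggers that are on and passes the all-on result to Mover.Move as a boolean.
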(event Custom|onTurned_イベント
  (params (on :type Boolean))
  (bind _on (CallFunction|Allon))
  (Default|Move (Variables|Default|Getmover) _on))

(event EventBeginPlay
  (for _array_element (Variables|Default|Gettriggers)
    (EventDispatchers|AssignOnTurned _array_element (delegate Custom|onTurned_イベント))))

(fn ConstructionScript)

(fn Allon
  (for _array_element (Variables|Default|Gettriggers)
    (if (Variables|/Game/Object/Movers/BP_Mover_Base.BP_Mover_Base_C|Geton _array_element)
      (LocalVariables|Setcounter (+ (LocalVariables|Getcounter) 1))))
  (return (== (Utilities|Array|Length (Variables|Default|Gettriggers)) (LocalVariables|Getcounter))))