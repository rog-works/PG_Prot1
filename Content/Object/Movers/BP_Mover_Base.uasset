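; BP_Mover_Base is a base Blueprint for mover objects that react to an on/off state from a TurnComponent.
; On BeginPlay it binds the component's begin-turned and turn-expired events, both of which pass their On value to ProcessMove.
; A separate Move function stores On before calling ProcessMove.
; ProcessMove only calls OnTurned with that state and contains no movement logic itself.
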(event Custom|onBeginTurned_イベント
  (params (on :type Boolean))
  (CallFunction|ProcessMove on))

(event Custom|onTurnExpired_イベント
  (params (on :type Boolean))
  (CallFunction|ProcessMove (Variables|Default|Geton)))

(event EventBeginPlay
  (bind _turncomponent (Variables|Default|GetTurnComponent))
  (Utilities|FlowControl|Sequence
    (:then_0
      (EventDispatchers|AssignOnBeginTurned _turncomponent (delegate Custom|onBeginTurned_イベント)))
    (:then_1
      (EventDispatchers|AssignOnTurnExpired _turncomponent (delegate Custom|onTurnExpired_イベント)))))

(fn ConstructionScript)

(fn Move
  (params (on :type Boolean))
  (bind _output_get (Variables|Default|Seton on))
  (CallFunction|ProcessMove _output_get))

(fn ProcessMove
  (params (on :type Boolean))
  (Default|CallOnTurned on))