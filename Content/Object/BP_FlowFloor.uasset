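; BP_FlowFloor is a floor actor that toggles between floating in place and physics-driven movement when shot.
; BeginPlay marks it as floating and saves its starting transform.
; A BP_Bullet sphere component overlapping its Box flips the Floating flag, either enabling physics simulation on the StaticMesh or disabling it and setting the actor back to the saved transform.
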(event OnComponentBeginOverlap(Box)
  (params (OverlappedComponent :type Primitive%20Component%20Object%20Reference) (OtherActor :type Actor%20Object%20Reference) (OtherComp :type Primitive%20Component%20Object%20Reference) (OtherBodyIndex :type Integer) (bFromSweep :type Boolean) (SweepResult :type Hit%20Result%20Structure%20%28by%20ref%29))
  (bind _staticmesh (Variables|Default|GetStaticMesh))
  (Utilities|IsValid OtherActor
    (:Is%20Valid
      (Utilities|Casting|CastToBP_Bullet OtherActor)
      (Utilities|Casting|CastToSphereComponent OtherComp)
      (if (Variables|Default|GetFloating)
        (Variables|Default|SetFloating false)
        (Physics|SetSimulatePhysics _staticmesh true)
        (else
          (Variables|Default|SetFloating true)
          (Physics|SetSimulatePhysics _staticmesh false)
          (Transformation|SetActorTransform (stale EventBeginPlay _output_get)))))))

(event EventBeginPlay
  (Variables|Default|SetFloating true)
  (bind _output_get (Variables|Default|SetNewVar_0 (Transformation|GetActorTransform))))

(fn ConstructionScript)