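; BP_Bullet is a bullet actor that detects hits by line trace and leaves a hit effect.
; It stores its spawn location, then every Tick traces on the Visibility channel from there to its current location.
; On a hit it spawns BP_NS_Hit at its current location rather than the impact point, yawed back toward the spawn point, and destroys itself.
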(event EventTick
  (params (DeltaSeconds :type Float%20%28single-precision%29))
  (bind _returnvalue (Transformation|GetActorLocation))
  (bind _spawnlocation (Variables|Default|GetSpawnLocation))
  (bind _returnvalue_2 (Math|Rotator|FindLookatRotation _spawnlocation _returnvalue))
  (bind _returnvalue_3 (Collision|LineTraceByChannel _spawnlocation _returnvalue "TraceTypeQuery1" false 0 "None"))
  (if _returnvalue_3
    (Game|SpawnActorfromClass "/Game/Effect/BP_NS_Hit.BP_NS_Hit_C" (Math|Transform|MakeTransform _returnvalue (Math|Rotator|MakeRotator (.roll _returnvalue_2) (.pitch _returnvalue_2) (+ (.yaw _returnvalue_2) 1.8e+02)) "1.000000,1.000000,1.000000") "Undefined" 0 0)
    (Actor|DestroyActor)))

(event EventBeginPlay
  (Variables|Default|SetSpawnLocation (Transformation|GetActorLocation)))

(fn ConstructionScript)