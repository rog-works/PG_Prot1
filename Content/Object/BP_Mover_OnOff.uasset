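; BP_Mover_OnOff slides a referenced MoveActor between its starting location and the location of a GuideActor, driven by an on/off state.
; BeginPlay caches both locations and enables movement only when both actors are valid.
; Move stores the On flag, then plays one of two timelines that lerp toward the guide or back.
; Each timeline plays from the start, so motion always begins at an endpoint.
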(event Custom|MoveForward
  (bind _新規track_0 (Timeline|タイムライン PlayFromStart)
    (:Update
      (Transformation|SetActorLocation (Variables|Default|GetmoveActor) (Math|Vector|Lerp(Vector) (Variables|Default|GetinitialObject) (Variables|Default|GetinitialGuide) _新規track_0) false false))))

(event Custom|MoveBackward
  (bind _新規track_0 (Timeline|タイムライン_1 PlayFromStart)
    (:Update
      (Transformation|SetActorLocation (Variables|Default|GetmoveActor) (Math|Vector|Lerp(Vector) (Variables|Default|GetinitialGuide) (Variables|Default|GetinitialObject) _新規track_0) false false))))

(event Custom|MoveStart
  (if (Variables|Default|Getenabled)
    (if (Variables|Default|Geton)
      (CallFunction|MoveForward)
      (else
        (CallFunction|MoveBackward)))))

(event EventBeginPlay
  (bind _moveactor (Variables|Default|GetmoveActor))
  (bind _guideactor (Variables|Default|GetguideActor))
  (Utilities|IsValid _guideactor
    (:Is%20Valid
      (Utilities|IsValid _moveactor
        (:Is%20Valid
          (Variables|Default|SetinitialGuide (Transformation|GetActorLocation _guideactor))
          (Variables|Default|SetinitialObject (Transformation|GetActorLocation _moveactor))
          (Variables|Default|Setenabled true))))))

(fn ConstructionScript)

(fn Move
  (params (on :type Boolean))
  (Variables|Default|Seton on)
  (CallFunction|MoveStart))