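; Interactive light that toggles on interaction and is temporarily forced on when a BP_Bullet sphere hits its box.
; Tick counts down the override, truncating so it drops about one per frame, while a screen-projected UI_ModEffected widget shows progress.
; GetLightOn prefers the override over the toggled state, and changes drive TurnLightOn, which sets point light intensity and dynamic-material emissive power.
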(event OnComponentBeginOverlap(Box)
  (params (OverlappedComponent :type Primitive%20Component%20Object%20Reference) (OtherActor :type Actor%20Object%20Reference) (OtherComp :type Primitive%20Component%20Object%20Reference) (OtherBodyIndex :type Integer) (bFromSweep :type Boolean) (SweepResult :type Hit%20Result%20Structure%20%28by%20ref%29))
  (Utilities|IsValid OtherActor
    (:Is%20Valid
      (Utilities|Casting|CastToBP_Bullet OtherActor)
      (Utilities|Casting|CastToSphereComponent OtherComp)
      (Variables|Default|SetModPower (Utilities|Struct|MakeBPST_Power 60 true)))))

(event Custom|カスタムイベント
  (params (On :type Boolean))
  (if true
    (Variables|Default|SetRealLightOn (not (Variables|Default|GetRealLightOn)))))

(event EventBeginPlay
  (Utilities|FlowControl|Sequence
    (:then_0
      (bind _returnvalue (UserInterface|CreateWidget "/Game/UI/UI_ModEffected.UI_ModEffected_C"))
      (Variables|Default|SetUI_Effected _returnvalue)
      (Widget|SetVisibility _returnvalue "Hidden")
      (UserInterface|Viewport|AddtoViewport _returnvalue 0))
    (:then_1
      (EventDispatchers|BindEventtoOnInteract (delegate Custom|カスタムイベント)))))

(event EventTick
  (params (DeltaSeconds :type Float%20%28single-precision%29))
  (bind _ui_effected (Variables|Default|GetUI_Effected))
  (Utilities|FlowControl|Sequence
    (:then_0
      (if (> (Math|Float|Truncate (- (.dulation (Variables|Default|GetModPower)) DeltaSeconds)) 0)
        (Variables|Default|SetModPower (Utilities|Struct|MakeBPST_Power (Math|Float|Truncate (- (.dulation (Variables|Default|GetModPower)) DeltaSeconds)) true))
        (Utilities|FlowControl|Sequence
          (:then_0
            (Widget|SetVisibility _ui_effected "Visible")
            (Class|Widget|SetRenderTranslation (Variables|Default|GetUI_Effected) (.ScreenPosition (Class|WidgetLayoutLibrary|ProjectWorldLocationtoWidgetPosition (Game|GetPlayerController 0) (Transformation|GetActorLocation) false))))
          (:then_1
            (Variables|/Game/UI/UI_ModEffected.UI_ModEffected_C|Setprogress (Variables|Default|GetUI_Effected) (/ (Math|Conversions|ToFloat(Integer) (.dulation (Variables|Default|GetModPower))) 6e+01))))
        (else
          (Variables|Default|SetModPower (Utilities|Struct|MakeBPST_Power 0 true))
          (Widget|SetVisibility _ui_effected "Hidden"))))
    (:then_1
      (bind _on (CallFunction|GetLighton))
      (if (!= _on (Variables|Default|GetPrevLightOn))
        (CallFunction|TurnLighton _on)
        (Variables|Default|SetPrevLightOn _on)))))

(fn ConstructionScript
  (bind _returnvalue (Rendering|Material|CreateDynamicMaterialInstance (Variables|Default|GetStaticMesh) 0 0 "None" :!class /Script/Engine.PrimitiveComponent))
  (bind _output_get (Variables|Default|SetMI_Light _returnvalue))
  (Rendering|Material|SetVectorParameterValue _output_get "EmissiveColor" (Variables|Default|GetEmissiveColor) :!class /Script/Engine.MaterialInstanceDynamic)
  (CallFunction|TurnLighton (Variables|Default|GetRealLightOn)))

(fn TurnLighton
  (params (On :type Boolean))
  (bind _pointlight (Variables|Default|GetPointLight))
  (bind _mi_light (Variables|Default|GetMI_Light))
  (if On
    (Rendering|Material|SetScalarParameterValue _mi_light "EmissivePower" (Variables|Default|GetEmissivePower) :!class /Script/Engine.MaterialInstanceDynamic)
    (Rendering|Components|Light|SetIntensity _pointlight (Variables|Default|GetLightIntensity))
    (else
      (Rendering|Material|SetScalarParameterValue _mi_light "EmissivePower" 0.0 :!class /Script/Engine.MaterialInstanceDynamic)
      (Rendering|Components|Light|SetIntensity _pointlight 0.0))))

(fn GetLighton
  (if (> (.dulation (Variables|Default|GetModPower)) 0)
    (LocalVariables|SetResultOn (.on (Variables|Default|GetModPower)))
    (else
      (bind _output_get (LocalVariables|SetResultOn (Variables|Default|GetRealLightOn)))))
  (return _output_get))