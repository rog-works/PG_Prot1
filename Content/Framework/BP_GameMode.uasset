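; Game mode that owns the player's Statistics and Achievements and restores saved sessions.
; On BeginPlay it creates both objects, then binds the activity event, which updates statistics and prints any newly unlocked achievements.
; The load event reads the slot name from the options string and opens an SB_Save_Session.
; It matches the save point by display name, moves the character to its arrow, then restores jump and save-point statistics and achieved flags.
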(event Custom|OnLoad_イベント
  (bind _returnvalue (SaveGame|LoadGamefromSlot (.RightS (Utilities|String|Split (Variables|Default|GetOptionsString) "?"))))
  (bind _assb_save_session (Utilities|Casting|CastToSB_Save_Session _returnvalue))
  (Utilities|FlowControl|Sequence
    (:then_0
      (CallFunction|LoadPlayerLocation (.location (.player (Variables|/Game/Framework/Save/SB_Save_Session.SB_Save_Session_C|Getgame _assb_save_session)))))
    (:then_1
      (CallFunction|LoadPlayerTransform))
    (:then_2
      (CallFunction|LoadStatisticsPlayer (.player (.statistics (Variables|/Game/Framework/Save/SB_Save_Session.SB_Save_Session_C|Getgame _assb_save_session)))))
    (:then_3
      (CallFunction|LoadStatisticsObject (.object (.statistics (Variables|/Game/Framework/Save/SB_Save_Session.SB_Save_Session_C|Getgame _assb_save_session)))))
    (:then_4
      (CallFunction|LoadAchievements (.achievements (Variables|/Game/Framework/Save/SB_Save_Session.SB_Save_Session_C|Getgame _assb_save_session))))))

(event Custom|OnActivity_イベント
  (params (activity :type String))
  (Default|FireActivity (Variables|Default|GetStatistics) activity)
  (bind _achievements (Default|Unlock (Variables|Default|GetAchievements) (Variables|Default|GetStatistics)))
  (for _array_element _achievements
    (Development|PrintString (Utilities|GetDisplayName _array_element))))

(event EventBeginPlay
  (Utilities|FlowControl|Sequence
    (:then_0
      (bind _returnvalue (Game|ConstructObjectfromClass "/Game/Framework/Statistics/Statistics.Statistics_C"))
      (bind _output_get (Variables|Default|SetStatistics _returnvalue))
      (Default|Initialize _output_get)
      (bind _returnvalue_2 (Game|ConstructObjectfromClass "/Game/Framework/Statistics/Achievements.Achievements_C"))
      (bind _output_get_2 (Variables|Default|SetAchievements _returnvalue_2))
      (Default|Initialize _output_get_2)
      (EventDispatchers|AssignOnActivity (delegate Custom|OnActivity_イベント)))
    (:then_1
      (EventDispatchers|AssignOnLoad (delegate Custom|OnLoad_イベント)))))

(fn ConstructionScript)

(fn LoadPlayerTransform
  (bind _asbp_pg_character (Utilities|Casting|CastToBP_PG_Character (Game|GetPlayerCharacter 0)))
  (Utilities|IsValid (Variables|/Game/Character/BP_PG_Character.BP_PG_Character_C|GetActivateSavePoint _asbp_pg_character)
    (:Is%20Valid
      (Transformation|SetActorTransform _asbp_pg_character (Math|Transform|MakeTransform (Transformation|GetWorldLocation (Actor|GetComponentbyClass (Variables|/Game/Character/BP_PG_Character.BP_PG_Character_C|GetActivateSavePoint _asbp_pg_character) "/Script/Engine.ArrowComponent")) (Transformation|GetWorldRotation (Actor|GetComponentbyClass (Variables|/Game/Character/BP_PG_Character.BP_PG_Character_C|GetActivateSavePoint _asbp_pg_character) "/Script/Engine.ArrowComponent")) "1.000000,1.000000,1.000000")))))

(fn LoadPlayerLocation
  (params (inData :type Save%20Game%20Player%20Location%20Structure))
  (if (!= 0 (Utilities|String|Len (.name inData)))
    (bind _outactors (Actor|GetAllActorsOfClass "/Game/Object/BP_SavePoint.BP_SavePoint_C"))
    (for _array_element _outactors
      (bind _returnvalue (Class|PGP1GameModeBase|StringEqual (Utilities|GetDisplayName _array_element) (.name inData)))
      (if _returnvalue
        (bind _asbp_pg_character (Utilities|Casting|CastToBP_PG_Character (Game|GetPlayerCharacter 0)))
        (Default|SetActiveSavePoint _asbp_pg_character _array_element)))))

(fn LoadStatisticsPlayer
  (params (inData :type Save%20Game%20Statistics%20Player%20Structure))
  (bind _returnvalue (Game|ConstructObjectfromClass "/Game/Framework/Statistics/StatRecords/StatRecord_PlayerJumps.StatRecord_PlayerJumps_C"))
  (bind _path (Default|Path _returnvalue))
  (bind _asstat_record_player_jumps (Utilities|Casting|CastToStatRecord_PlayerJumps (.Value (Utilities|Map|Find (Variables|/Game/Framework/Statistics/Statistics.Statistics_C|Getrecords (Variables|Default|GetStatistics)) _path))))
  (bind _output_get (Variables|/Game/Framework/Statistics/StatRecords/StatRecord_PlayerJumps.StatRecord_PlayerJumps_C|Setjumps _asstat_record_player_jumps (.jumps inData)))
  (Development|PrintString (Utilities|String|Append "loading stat: " _path ": " (Utilities|String|ToString(Integer) _output_get))))

(fn LoadStatisticsObject
  (params (inData :type Save%20Game%20Statistics%20Object%20Structure))
  (bind _returnvalue (Game|ConstructObjectfromClass "/Game/Framework/Statistics/StatRecords/StatRecord_PerSavePointActivates.StatRecord_PerSavePointActivates_C"))
  (bind _path (Default|Path _returnvalue))
  (bind _asstat_record_per_save_point_activates (Utilities|Casting|CastToStatRecord_PerSavePointActivates (.Value (Utilities|Map|Find (Variables|/Game/Framework/Statistics/Statistics.Statistics_C|Getrecords (Variables|Default|GetStatistics)) _path))))
  (Utilities|Map|Clear (Variables|/Game/Framework/Statistics/StatRecords/StatRecord_PerSavePointActivates.StatRecord_PerSavePointActivates_C|Getactivates _asstat_record_per_save_point_activates))
  (bind _keys (Utilities|Map|Keys (.activates inData)))
  (for _array_element _keys
    (Utilities|Map|Add (Variables|/Game/Framework/Statistics/StatRecords/StatRecord_PerSavePointActivates.StatRecord_PerSavePointActivates_C|Getactivates _asstat_record_per_save_point_activates) _array_element (.Value (Utilities|Map|Find (.activates inData) _array_element)))
    (Development|PrintString (Utilities|String|Append "loading stat: " _array_element ": " _path "." _array_element (Utilities|String|ToString(Integer) (.Value (Utilities|Map|Find (.activates inData) _array_element)))))))

(fn LoadAchievements
  (params (inData :type Array%20of%20Strings))
  (for _array_element inData
    (if (.ReturnValue (Utilities|Map|Find (Variables|/Game/Framework/Statistics/Achievements.Achievements_C|Getrecords (Variables|Default|GetAchievements)) _array_element))
      (Variables|/Game/Framework/Statistics/Achievement.Achievement_C|Setachieved (.Value (Utilities|Map|Find (Variables|/Game/Framework/Statistics/Achievements.Achievements_C|Getrecords (Variables|Default|GetAchievements)) _array_element)) true)
      (Development|PrintString (Utilities|String|Append "loading achivement: " _array_element)))))